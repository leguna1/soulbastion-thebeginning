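; BP_Door is a passcode-protected door that swings open and closes itself automatically.
; TryOpenDoor compares the given code to Passcode and, if the door is not already open, sets IsOpen and calls ChangeDoorState.
; A timeline drives DoorMesh yaw, then after a delay clears IsOpen and reverses to close the door.
; The player reference cached on BeginPlay feeds a frame hit check that currently does nothing.
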(event OnComponentHit(SM_DoorFrame)
  (params (HitComponent :type Primitive%20Component%20Object%20Reference) (OtherActor :type Actor%20Object%20Reference) (OtherComp :type Primitive%20Component%20Object%20Reference) (NormalImpulse :type Vector :default "0, 0, 0") (Hit :type Hit%20Result%20Structure%20%28by%20ref%29))
  (bind _playercharacter (Variables|Default|GetPlayerCharacter)
    (:then
      (if (== _playercharacter OtherActor)
        _))
    (:else)))

(event Custom|ChangeDoorState
  (bind _alpha (Timeline|DoorTimeline PlayFromStart)
    (:Update
      (Transformation|SetRelativeRotation (Variables|Default|GetDoorMesh) (Math|Rotator|MakeRotator 0.0 0.0 _alpha) false false))
    (:Finished
      (if (Variables|Default|GetbIsOpen)
        (Utilities|FlowControl|Delay 5.0)
        (Variables|Default|SetbIsOpen false)
        (Timeline|DoorTimeline ReverseFromEnd)))))

(event EventBeginPlay
  (bind _returnvalue (Actor|GetActorOfClass "/Game/BP_Player.BP_Player_C"))
  (Variables|Default|SetPlayerCharacter _returnvalue))

(fn ConstructionScript)

(fn TryOpenDoor
  (params (InPasscode :type Integer))
  (if (and (== InPasscode (Variables|Default|GetPasscode)) (not (Variables|Default|GetbIsOpen)))
    (Variables|Default|SetbIsOpen true)
    (CallFunction|ChangeDoorState)))