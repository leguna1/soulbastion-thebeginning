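; BP_Ladder is a ladder actor built procedurally from a configurable number of stacked step meshes.
; The construction script destroys earlier steps, adds static mesh components at fixed height intervals, and moves BottomPoint and TopPoint to the first and last steps in CreatedLadders.
; GetSelectedTarget returns the ladder itself with a target type enum.
; BeginPlay prints debug checks that both points match their end steps' world locations.
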(event EventBeginPlay
  (bind _created_ladders (Variables|Default|GetCreated%20Ladders))
  (Development|PrintString (Utilities|String|ToString(Boolean) (Class|KismetMathLibrary|EqualExactlyVectorVector (Transformation|GetWorldLocation (Utilities|Array|Get(acopy) (Variables|Default|GetCreated%20Ladders))) (Transformation|GetWorldLocation (Variables|Default|GetBottomPoint)))))
  (Development|PrintString (Utilities|String|ToString(Boolean) (Class|KismetMathLibrary|EqualExactlyVectorVector (Transformation|GetWorldLocation (Utilities|Array|Get(acopy) _created_ladders (Utilities|Array|LastIndex _created_ladders))) (Transformation|GetWorldLocation (Variables|Default|GetTopPoint)))) true true "(R=0.202270,G=0.000000,B=1.000000,A=1.000000)"))

(fn ConstructionScript
  (bind _created_ladders (Variables|Default|GetCreated%20Ladders))
  (for _array_element (Variables|Default|GetCreated%20Ladders)
    (Components|DestroyComponent _array_element))
  (for _index (range 0 (- (Variables|Default|GetLadder%20Step%20Count) 1))
    (bind _returnvalue (AddComponent|AddStaticMeshComponent false (Math|Transform|MakeTransform (Math|Vector|MakeVector 0.0 0.0 (* _index (Variables|Default|GetHeigth))))))
    (bind _returnvalue_2 (Components|StaticMesh|SetStaticMesh _returnvalue (Variables|Default|GetNew%20Mesh)))
    (if _returnvalue_2
      (Utilities|Array|AddUnique (Variables|Default|GetCreated%20Ladders) _returnvalue)
      (Transformation|SetRelativeLocation (Variables|Default|GetBottomPoint) (Variables|/Script/Engine.SceneComponent|GetRelativeLocation (Utilities|Array|Get(acopy) (Variables|Default|GetCreated%20Ladders))) false false)
      (Transformation|SetRelativeLocation (Variables|Default|GetTopPoint) (Variables|/Script/Engine.SceneComponent|GetRelativeLocation (Utilities|Array|Get(acopy) _created_ladders (Utilities|Array|LastIndex _created_ladders))) false false))))

(fn GetSelectedTarget
  (return self "NewEnumerator2"))