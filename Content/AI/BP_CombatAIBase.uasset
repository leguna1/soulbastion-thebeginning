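; Base Blueprint for combat AI characters, providing a floating health bar, floating damage numbers and an empty PerformAttack function.
; On BeginPlay it configures both widgets, caches its AI controller and binds to the player camera's target-change event.
; The health bar shows only while the player targets this AI.
; StatSystem changes to the Health tag feed their delta to the damage number widget.
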(event OnStatChanged(StatSystem)
  (params (StatEvent :type Stat%20Changed%20Event%20Structure))
  (if (GameplayTags|MatchesTag (.stattag StatEvent) "(TagName=\"Stat.Health\")" true)
    (Default|ShowFloatingDamage (Variables|Default|GetAs%20WB%20Damage%20Amount) (.delta StatEvent))))

(event Custom|OnPlayerTarget
  (params (NewTarget :type Actor%20Object%20Reference))
  (Widget|SetVisibility (Variables|Default|GetAs%20WB%20Progressbar) (select (== NewTarget self) "Visible" "Hidden")))

(event EventBeginPlay
  (|CallParentFunction)
  (CallFunction|InitalSetup))

(fn ConstructionScript)

(fn InitalSetup
  (Utilities|FlowControl|Sequence
    (:then_0
      (bind _asbp_player (Utilities|Casting|CastToBP_Player (Game|GetPlayerCharacter 0)))
      (bind _output_get (Variables|Default|SetPlayer%20Camera (Actor|GetComponentbyClass _asbp_player "/Script/SoulBastion.PlayerCamera")))
      (EventDispatchers|BindEventtoOnTargetChanged _output_get (EventDispatchers|CreateEvent :!event Custom|OnPlayerTarget)))
    (:then_1
      (bind _healthbar (Variables|Default|GetHealthbar)
        (:then
          (bind _aswb_floating_progressbar (Utilities|Casting|CastToWB_FloatingProgressbar (UserInterface|GetWidget _healthbar)))
          (Variables|/Game/UI/Combat/WB_FloatingProgressbar.WB_FloatingProgressbar_C|SetStatComp _aswb_floating_progressbar (Variables|Default|GetStatSystem))
          (bind _output_get_2 (Variables|Default|SetAs%20WB%20Progressbar _aswb_floating_progressbar))
          (Variables|/Game/UI/Combat/WB_FloatingProgressbar.WB_FloatingProgressbar_C|SetStat%20Tag _output_get_2 "(TagName=\"Stat.Health\")")
          (Widget|SetVisibility _aswb_floating_progressbar "Hidden")
          (Variables|/Game/UI/Combat/WB_FloatingProgressbar.WB_FloatingProgressbar_C|SetNameText _aswb_floating_progressbar (Variables|Default|GetDisplayName)))
        (:else)))
    (:then_2
      (bind _damage (Variables|Default|GetDamage)
        (:then
          (bind _aswb_damage_amount (Utilities|Casting|CastToWB_DamageAmount (UserInterface|GetWidget _damage)))
          (Variables|Default|SetAs%20WB%20Damage%20Amount _aswb_damage_amount))
        (:else)))
    (:then_3
      (bind _asbp_aicontroller (Utilities|Casting|CastToBP_AIController (Pawn|GetController)))
      (Variables|Default|SetAs%20BP%20AIController _asbp_aicontroller))))

(fn PerformAttack
  (params (Montage%20To%20Play :type Anim%20Montage%20Object%20Reference) (Bonus%20Damage :type Float%20%28double-precision%29) (Hit%20FX :type Fx%20Data%20Structure)))