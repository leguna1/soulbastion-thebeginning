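; Player controller that creates the HUD, adds the default Enhanced Input mapping context and turns player input into ability requests.
; Input actions send gameplay tags to the controlled pawn through TryActivateAbilityMessage for attack, dash, block and other abilities.
; Block also forwards press and release, with elapsed time on press.
; Left Ctrl flip-flops cursor visibility and input mode between Game-and-UI and UI-only focused on the HUD.
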(event Input|EnhancedActionEvents|EnhancedInputActionIA_LightAttack
  (params (ActionValue :type Boolean) (ElapsedSeconds :type Float%20%28double-precision%29) (TriggeredSeconds :type Float%20%28double-precision%29) (InputAction :type Input%20Action%20Object%20Reference :default "/Game/Input/Actions/IA_LightAttack.IA_LightAttack"))
  (Class|BPICharacter|TryActivateAbility(Message) (Pawn|GetControlledPawn) "(TagName=\"Character.Ability.Attack.Light\")"))

(event Input|EnhancedActionEvents|EnhancedInputActionIA_Block
  (params (ActionValue :type Boolean) (ElapsedSeconds :type Float%20%28double-precision%29) (TriggeredSeconds :type Float%20%28double-precision%29) (InputAction :type Input%20Action%20Object%20Reference :default "/Game/Input/Actions/IA_Block.IA_Block"))
  (:Started
    (Class|BPICharacter|TryActivateAbility(Message) (Pawn|GetControlledPawn) "(TagName=\"Ability.Block\")" (Utilities|Struct|MakeMyPlayerInput "Pressed" "(X=0.000000,Y=0.000000)" ElapsedSeconds)))
  (:Completed
    (Class|BPICharacter|TryActivateAbility(Message) (Pawn|GetControlledPawn) "(TagName=\"Ability.Block\")" (Utilities|Struct|MakeMyPlayerInput "Released" "(X=0.000000,Y=0.000000)" 0.0))))

(event Input|EnhancedActionEvents|EnhancedInputActionIA_Dash
  (params (ActionValue :type Boolean) (ElapsedSeconds :type Float%20%28double-precision%29) (TriggeredSeconds :type Float%20%28double-precision%29) (InputAction :type Input%20Action%20Object%20Reference :default "/Game/Input/Actions/IA_Dash.IA_Dash"))
  (Class|BPICharacter|TryActivateAbility(Message) (Pawn|GetControlledPawn) "(TagName=\"Character.Ability.Mobility.Dash\")"))

(event Input|EnhancedActionEvents|EnhancedInputActionIA_Z
  (params (ActionValue :type Boolean) (ElapsedSeconds :type Float%20%28double-precision%29) (TriggeredSeconds :type Float%20%28double-precision%29) (InputAction :type Input%20Action%20Object%20Reference :default "/Game/Input/Actions/IA_Z.IA_Z"))
  (Class|BPICharacter|TryActivateAbility(Message) (Pawn|GetControlledPawn) "(TagName=\"Ability.CrimsonVial\")"))

(event Input|EnhancedActionEvents|EnhancedInputActionIA_X
  (params (ActionValue :type Boolean) (ElapsedSeconds :type Float%20%28double-precision%29) (TriggeredSeconds :type Float%20%28double-precision%29) (InputAction :type Input%20Action%20Object%20Reference :default "/Game/Input/Actions/IA_X.IA_X"))
  (Class|BPICharacter|TryActivateAbility(Message) (Pawn|GetControlledPawn) "(TagName=\"Ability.Energize\")"))

(event EventBeginPlay
  ;[0.15 0.15 0.15 0.5] Initialize player input
  ;;[0.15 0.15 0.15 0.5] Add regular input mappings
  (if (Pawn|IsLocalPlayerController)
    (bind _returnvalue (UserInterface|CreateWidget "/Game/UI/WB_HUD.WB_HUD_C" self))
    (bind _output_get (Variables|Default|SetPlayer%20HUD _returnvalue))
    (UserInterface|Viewport|AddtoViewport _output_get 0)
    (Input|SetInputModeGameOnly self false)
    (Input|AddMappingContext (PlayerController|LocalPlayerSubsystems|GetEnhancedInputLocalPlayerSubsystem) "/Game/Input/IMC_Default.IMC_Default" 0 "(bIgnoreAllPressedKeysUntilRelease=True,bForceImmediately=False,bNotifyUserSettings=False)")))

(event Input|KeyboardEvents|LeftCtrl
  (params (Key :type Key%20Structure :default "None"))
  (:Pressed
    (Utilities|FlowControl|FlipFlop
      (:A
        (Variables|Default|SetbShowMouseCursor false)
        (Input|SetInputModeGameandUI self (Variables|Default|GetPlayer%20HUD) "DoNotLock" true false))
      (:B
        (Variables|Default|SetbShowMouseCursor true)
        (Input|SetInputModeUIOnly self (Variables|Default|GetPlayer%20HUD) "LockAlways" false)))))

(fn ConstructionScript)