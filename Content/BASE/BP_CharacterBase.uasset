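; Base character Blueprint that provides shared stats, abilities, targeting, faction checks and movement for characters.
; Stat, life, essence, hit and skill calls forward to StatSystem and AbilitySystem components, with activation confirmed by matching the active skill's tag.
; SetMoveMode, applied at BeginPlay, maps gait presets onto CharacterMovement, and ToggleRagdoll switches mesh physics and reattaches it to the capsule.
; Several getters, including player controller, HUD, weapon sockets and move mode, are empty stubs.
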(event EventBeginPlay
  (CallFunction|SetMoveMode (Variables|Character|GetMovement%20Mode) 0.0))

(fn ConstructionScript)

(fn AdjustMovementSettings
  (params (Max%20Walk%20Speed :type Float%20%28double-precision%29) (Modify%20Walk%20Speed%20Value :type Float%20%28double-precision%29) (Acceleration :type Float%20%28double-precision%29) (BrakingDecel%20 :type Float%20%28double-precision%29) (RotationRate%20 :type Float%20%28double-precision%29) (Orient%20Rotation%20to%20Movement :type Boolean) (Use%20Controller%20Desired%20Rotation :type Boolean))
  (bind _charactermovement (Variables|Character|GetCharacterMovement))
  (Variables|/Script/Engine.CharacterMovementComponent|SetMaxWalkSpeed _charactermovement (Math|Float|Clamp(Float) (+ Max%20Walk%20Speed Modify%20Walk%20Speed%20Value) 0.0 1e+04))
  (Variables|/Script/Engine.CharacterMovementComponent|SetMaxAcceleration _charactermovement Acceleration)
  (Variables|/Script/Engine.CharacterMovementComponent|SetBrakingDecelerationWalking _charactermovement BrakingDecel%20)
  (Variables|/Script/Engine.CharacterMovementComponent|SetRotationRate _charactermovement (Math|Rotator|MakeRotator 0.0 0.0 RotationRate%20))
  (Variables|/Script/Engine.CharacterMovementComponent|SetbOrientRotationToMovement _charactermovement Orient%20Rotation%20to%20Movement)
  (Variables|/Script/Engine.CharacterMovementComponent|SetbUseControllerDesiredRotation _charactermovement Use%20Controller%20Desired%20Rotation)
  (return Max%20Walk%20Speed))

(fn ActivateAbilitybyTag
  (params (Skill%20Tag :type Gameplay%20Tag%20Structure))
  (bind _abilitysystem (Variables|Default|GetAbilitySystem))
  (bind (_returnvalue _instance) (Class|AbilitySystem|GetCurrentlyActiveSkill _abilitysystem))
  (Class|AbilitySystem|TryActivateAbility :self _abilitysystem :SkillTag Skill%20Tag :Input "Tap")
  (if _returnvalue
    (return (GameplayTags|MatchesTag (Variables|/Script/SoulBastion.SkillBase|GetSkillTag _instance) Skill%20Tag true))))

(fn GetCurrentTarget
  (bind _current_target (Variables|Character|GetCurrent%20Target))
  (bind _type (Class|BPITargetable|GetTargetType(Message) _current_target))
  (return _current_target _type))

(fn GetFactionName
  (return (Variables|Character|GetFaction%20Name)))

(fn GetMainWeaponSockets
  (return 0 0))

(fn GetMoveMode
  (return "NewEnumerator0"))

(fn GetPlayerController
  (return 0))

(fn GetPlayerHUD
  (return 0))

(fn GetSoulForce
  (return 0.0))

(fn GetStatValue
  (params (Stat :type Gameplay%20Tag%20Structure) (Type :type EStatValueType%20Enum :default "None"))
  (return (Class|StatSystem|GetStatValue (Variables|Default|GetStatSystem) Stat Type)))

(fn GetTargetType
  (return (Variables|Default|GetTargetable%20Type)))

(fn GetUtilityBox
  (return (Variables|Default|GetUtilityBox)))

(fn GrantSoulEssence
  (params (Amount :type Float%20%28double-precision%29))
  (Class|StatSystem|GainEssence (Variables|Default|GetStatSystem) Amount)
  (return))

(fn HitResponse
  (params (Hit%20Info :type Hit%20Info%20Structure))
  (Class|AbilitySystem|HitResponse (Variables|Default|GetAbilitySystem) Hit%20Info)
  (return true))

(fn IsAlive
  (return (Class|StatSystem|IsAlive (Variables|Default|GetStatSystem))))

(fn IsEnemy
  (params (Other%20Actor :type Actor%20Object%20Reference))
  (bind _return (Class|BPICharacter|GetFactionName(Message) Other%20Actor))
  (return (!= _return (Variables|Character|GetFaction%20Name))))

(fn ModifyStat
  (params (Modifier%20Source :type Actor%20Object%20Reference) (StatTag :type Gameplay%20Tag%20Structure) (Type :type EStatValueType%20Enum :default "None") (ModifyValue :type Float%20%28double-precision%29))
  (Class|StatSystem|ModifyStat (Variables|Default|GetStatSystem) Modifier%20Source StatTag Type ModifyValue)
  (return true))

(fn SetCurrentTarget
  (params (Actor :type Actor%20Object%20Reference))
  (Variables|Character|SetCurrent%20Target Actor)
  (return))

(fn SetMoveMode
  (params (Mode :type E_GroundSpeedMode%20Enum :default "NewEnumerator0") (Modify%20Value :type Float%20%28double-precision%29))
  (Variables|Default|SetOld%20Movement%20Mode (Variables|Character|GetMovement%20Mode))
  (bind _output_get (Variables|Character|SetMovement%20Mode Mode))
  (switch Utilities|FlowControl|Switch|SwitchonE_GroundSpeedMode _output_get
    (:NewEnumerator0
      (bind _new_speed (CallFunction|AdjustMovementSettings 0.0 Modify%20Value 0.0 0.0 2.6e+02 true false))
      (return _new_speed))
    (:NewEnumerator1
      (bind _new_speed_2 (CallFunction|AdjustMovementSettings 2.5e+02 Modify%20Value 8e+02 1e+03 3.6e+02 false true))
      (return _new_speed_2))
    (:NewEnumerator2
      (bind _new_speed_3 (CallFunction|AdjustMovementSettings 4e+02 Modify%20Value 1.4e+03 1.7e+03 5e+02 true false))
      (return _new_speed_3))
    (:NewEnumerator3
      (bind _new_speed_4 (CallFunction|AdjustMovementSettings 5e+02 Modify%20Value 2e+03 2.5e+03 5.5e+02 true false))
      (return _new_speed_4))
    (:NewEnumerator4
      (bind _new_speed_5 (CallFunction|AdjustMovementSettings 7e+02 Modify%20Value 2.8e+03 3.5e+03 6.5e+02 true false))
      (return _new_speed_5))))

(fn ToggleLifeState
  (params (bIsAlive :type Boolean))
  (Variables|/Script/SoulBastion.StatSystem|SetbIsAlive (Variables|Default|GetStatSystem) bIsAlive)
  (return))

(fn ToggleRagdoll
  (params (Ragdoll :type Boolean))
  (bind _capsulecomponent (Variables|Collision|GetCapsuleComponent))
  (bind _mesh (Variables|Character|GetMesh))
  (bind _returnvalue (Transformation|GetWorldRotation _capsulecomponent))
  (if Ragdoll
    (Physics|SetSimulatePhysics (Variables|Character|GetMesh) true)
    (Collision|SetCollisionEnabled (Variables|Collision|GetCapsuleComponent) "NoCollision")
    (return)
    (else
      (Physics|SetSimulatePhysics (Variables|Character|GetMesh) false)
      (Collision|SetCollisionEnabled (Variables|Collision|GetCapsuleComponent) "QueryAndPhysics")
      (Transformation|SetWorldLocationAndRotation _mesh (- (Transformation|GetWorldLocation _capsulecomponent) "0.000000,0.000000,89.000000") (Math|Rotator|MakeRotator (.roll _returnvalue) (.pitch _returnvalue) (- (.yaw _returnvalue) 89.0)) false false)
      (Transformation|AttachComponentToComponent _mesh (Variables|Collision|GetCapsuleComponent) "pelvis" "KeepWorld" "KeepWorld" "KeepWorld" true)
      (if (Rendering|IsVisible (Variables|Character|GetMesh))
        _
        (else
          (Rendering|SetVisibility (Variables|Character|GetMesh) true true)))
      (return))))

(fn TryActivateAbility
  (params (Skill%20Tag :type Gameplay%20Tag%20Structure) (Input :type EActivationInput%20Enum :default "Tap") (Input%20Action :type Vector%202D%20Structure))
  (bind _abilitysystem (Variables|Default|GetAbilitySystem))
  (bind (_returnvalue _instance) (Class|AbilitySystem|GetCurrentlyActiveSkill _abilitysystem))
  (Class|AbilitySystem|TryActivateAbility _abilitysystem Skill%20Tag Input Input%20Action 0.0)
  (if _returnvalue
    (return (GameplayTags|MatchesTag (Variables|/Script/SoulBastion.SkillBase|GetSkillTag _instance) Skill%20Tag true))))